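; Night-time melee enemy AI that chases whichever of two players is closer in 2D distance and destroys itself when the sky timer reports night is over.
; A looping AIMoveTo replays the attack montage and, on reaching a player not too far above, deals damage gated by a delayed DoOnce.
; Taking damage updates its health bar and briefly staggers it; death credits the killer and randomly drops a health pickup.
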(event Custom|UpdateHealth
  (params (PlayerDamage :type Float%20%28double-precision%29) (Player :type BP%20Third%20Person%20Character%20Synty%20Object%20Reference))
  ;[1 1 1] UpdateHealth then kill
  (bind _output_get (Variables|Default|SetCurrentHealth (- (Variables|Default|GetCurrentHealth) PlayerDamage)))
  (if (<= _output_get 0.0)
    (Default|AddKill Player 2)
    (switch int (Math|Random|RandomInteger 2)
      (:Default
        _)
      (:0
        (Game|SpawnActorfromClass "/Game/Tyler/Bluebrints/BP_HealthPickUp.BP_HealthPickUp_C" (Transformation|GetWorldTransform (Variables|Collision|GetCapsuleComponent self)) "Undefined" "MultiplyWithRoot" 0 0))
      (:1
        _)
      (:2
        _))
    (Actor|DestroyActor)
    (else
      (CallFunction|AddStagger)
      (CallFunction|UpdateHealthWidget))))

(event Custom|AddStagger
  (bind _charactermovement (Variables|Character|GetCharacterMovement))
  ;[1 1 1] Enemy Stagger
  (Variables|/Script/Engine.CharacterMovementComponent|SetMaxWalkSpeed _charactermovement 0.0)
  (Utilities|FlowControl|Delay 0.25)
  (Variables|/Script/Engine.CharacterMovementComponent|SetMaxWalkSpeed _charactermovement 3e+02))

(event Custom|UpdateHealthWidget
  ;[1 1 1] Update the health on the widget
  (bind _asw_enemy_health (Utilities|Casting|CastToW_EnemyHealth (UserInterface|GetUserWidgetObject (Variables|Default|GetHealthBar))))
  (Default|UpdateHealthBar _asw_enemy_health (Variables|Default|GetCurrentHealth) (Variables|Default|GetMaxHealth)))

(event EventBeginPlay
  (bind _self self)
  (bind _capsulecomponent (Variables|Collision|GetCapsuleComponent _self))
  (bind _returnvalue (Transformation|GetWorldLocation _capsulecomponent))
  ;[1 1 1] Enemy Move
  ;;[1 1 1] Ref to sky timer
  (bind _outactors (Actor|GetAllActorsOfClass "/Game/Tyler/Bluebrints/Bp_SkyTimer.Bp_SkyTimer_C"))
  (Variables|Default|SetSkyTimerRef (Utilities|Array|Get(acopy) _outactors))
  (bind _outactors_2 (Actor|GetAllActorsOfClass "/Game/ThirdPerson/Blueprints/BP_ThirdPersonCharacterSynty.BP_ThirdPersonCharacterSynty_C"))
  (AI|AIMoveTo self "0, 0, 0" (select (> (Math|Vector|Distance(Vector) (Math|Vector|MakeVector (.x _returnvalue) (.y _returnvalue) 0.0) (Math|Vector|MakeVector (.x (Transformation|GetWorldLocation (Variables|/Script/Engine.Character|GetCapsuleComponent (Utilities|Array|Get(acopy) _outactors_2)))) (.y (Transformation|GetWorldLocation (Variables|/Script/Engine.Character|GetCapsuleComponent (Utilities|Array|Get(acopy) _outactors_2)))) 0.0)) (Math|Vector|Distance(Vector) (Math|Vector|MakeVector (.x _returnvalue) (.y _returnvalue) 0.0) (Math|Vector|MakeVector (.x (Transformation|GetWorldLocation (Variables|/Script/Engine.Character|GetCapsuleComponent (Utilities|Array|Get(acopy) _outactors_2 1)))) (.y (Transformation|GetWorldLocation (Variables|/Script/Engine.Character|GetCapsuleComponent (Utilities|Array|Get(acopy) _outactors_2 1)))) 0.0))) (Utilities|Array|Get(acopy) _outactors_2 1) (Utilities|Array|Get(acopy) _outactors_2)) 2.0 false :!label _label
    (:then
      (Utilities|FlowControl|Delay 1.0 :!label _label_2)
      (Animation|PlayAnimMontage "/Game/Developers/dynod/Attack.Attack" 1.0 "None")
      (goto _label))
    (:OnSuccess
      (if (not (> (.z (Transformation|GetWorldLocation (Variables|/Script/Engine.Actor|GetRootComponent (select (> (Math|Vector|Distance(Vector) (Math|Vector|MakeVector (.x _returnvalue) (.y _returnvalue) 0.0) (Math|Vector|MakeVector (.x (Transformation|GetWorldLocation (Variables|/Script/Engine.Character|GetCapsuleComponent (Utilities|Array|Get(acopy) _outactors_2)))) (.y (Transformation|GetWorldLocation (Variables|/Script/Engine.Character|GetCapsuleComponent (Utilities|Array|Get(acopy) _outactors_2)))) 0.0)) (Math|Vector|Distance(Vector) (Math|Vector|MakeVector (.x _returnvalue) (.y _returnvalue) 0.0) (Math|Vector|MakeVector (.x (Transformation|GetWorldLocation (Variables|/Script/Engine.Character|GetCapsuleComponent (Utilities|Array|Get(acopy) _outactors_2 1)))) (.y (Transformation|GetWorldLocation (Variables|/Script/Engine.Character|GetCapsuleComponent (Utilities|Array|Get(acopy) _outactors_2 1)))) 0.0))) (Utilities|Array|Get(acopy) _outactors_2 1) (Utilities|Array|Get(acopy) _outactors_2))))) (+ (.z (Transformation|GetWorldLocation (Variables|Collision|GetCapsuleComponent))) 2e+02))) ; check player hight
        (Utilities|FlowControl|DoOnce false :!label _label_3
          (:Completed
            (if (> (Math|Vector|Distance(Vector) (Math|Vector|MakeVector (.x _returnvalue) (.y _returnvalue) 0.0) (Math|Vector|MakeVector (.x (Transformation|GetWorldLocation (Variables|/Script/Engine.Character|GetCapsuleComponent (Utilities|Array|Get(acopy) _outactors_2)))) (.y (Transformation|GetWorldLocation (Variables|/Script/Engine.Character|GetCapsuleComponent (Utilities|Array|Get(acopy) _outactors_2)))) 0.0)) (Math|Vector|Distance(Vector) (Math|Vector|MakeVector (.x _returnvalue) (.y _returnvalue) 0.0) (Math|Vector|MakeVector (.x (Transformation|GetWorldLocation (Variables|/Script/Engine.Character|GetCapsuleComponent (Utilities|Array|Get(acopy) _outactors_2 1)))) (.y (Transformation|GetWorldLocation (Variables|/Script/Engine.Character|GetCapsuleComponent (Utilities|Array|Get(acopy) _outactors_2 1)))) 0.0))) ; Player 2 true, player 1 false
              ;;[1 1 1] Damage
              (Default|TakeDamage (Utilities|Array|Get(acopy) _outactors_2 1) 1e+01) ; Player 2
              (else
                (Default|TakeDamage (Utilities|Array|Get(acopy) _outactors_2) 1e+01) ; Player one
              ))
            (Utilities|FlowControl|Delay 1.0)
            (goto _label_3 Reset)))))
    (:OnFail
      (goto _label_2))))

(event EventTick
  (params (DeltaSeconds :type Float%20%28single-precision%29))
  ;[1 1 1] Check if day
  (Utilities|FlowControl|Delay 1.0)
  (if (not (Variables|/Game/Tyler/Bluebrints/Bp_SkyTimer.Bp_SkyTimer_C|GetNightTimer (Variables|Default|GetSkyTimerRef)))
    (Actor|DestroyActor)))

(fn ConstructionScript)
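; Player sword that attaches to the Synty third-person character's weapon socket on pickup and upgrades twice as the player's Helps count rises.
; AddSword stores the player, disables collision and sets starting PlayerDamage.
; Tick, throttled by a Delay, compares Helps to HelpsReq, calls SwordUpgrade, then resets the threshold.
; SwordUpgrade reveals the next mesh and raises player damage, repeating the final tier while the threshold remains met.
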(event Custom|SwordUpgrade
  ;[1 1 1] Both sword upgrades
  (if (Variables|Default|GetFirstUpgrade)
    (Rendering|SetVisibility (Variables|Default|GetSM_Wep_Wooden_01) false false)
    (Rendering|SetVisibility (Variables|Default|GetSM_Wep_Shortsword_02) true false)
    (bind _output_get (Variables|Default|SetSwordDamage 5e+01))
    (Variables|/Game/ThirdPerson/Blueprints/BP_ThirdPersonCharacterSynty.BP_ThirdPersonCharacterSynty_C|SetPlayerDamage (Variables|Default|Getref%20to%20Player) _output_get)
    (Variables|Default|SetFirstUpgrade false)
    (else
      (Rendering|SetVisibility (Variables|Default|GetN_SwordUpgrade) true false)
      (bind _output_get_2 (Variables|Default|SetSwordDamage 1e+02))
      (Variables|/Game/ThirdPerson/Blueprints/BP_ThirdPersonCharacterSynty.BP_ThirdPersonCharacterSynty_C|SetPlayerDamage (Variables|Default|Getref%20to%20Player) _output_get_2))))

(event Custom|AddSword
  (params (Player :type Actor%20Object%20Reference))
  ;[1 1 1] Sword Pick up
  (bind _asbp_third_person_character_synty (Utilities|Casting|CastToBP_ThirdPersonCharacterSynty Player))
  (Variables|Default|Setref%20to%20Player _asbp_third_person_character_synty)
  (Variables|Default|SetSwordPickedUp true)
  (Collision|SetCollisionEnabled (Variables|Default|GetSM_Wep_Wooden_01) "NoCollision")
  (Transformation|AttachComponentToComponent (Variables|/Game/ThirdPerson/Blueprints/BP_ThirdPersonCharacterSynty.BP_ThirdPersonCharacterSynty_C|GetWeaponSocket _asbp_third_person_character_synty) "None" "SnapToTarget" "SnapToTarget" "SnapToTarget" true)
  (Variables|/Game/ThirdPerson/Blueprints/BP_ThirdPersonCharacterSynty.BP_ThirdPersonCharacterSynty_C|SetPlayerDamage _asbp_third_person_character_synty 2e+01))

(event Collision|EventActorBeginOverlap
  (params (OtherActor :type Actor%20Object%20Reference)))

(event EventTick
  (params (DeltaSeconds :type Float%20%28single-precision%29))
  ;[1 1 1] Sword Upgrade on helps
  (Utilities|FlowControl|Delay 0.2)
  (if (Variables|Default|GetSwordPickedUp)
    (if (>= (Variables|/Game/ThirdPerson/Blueprints/BP_ThirdPersonCharacterSynty.BP_ThirdPersonCharacterSynty_C|GetHelps (Variables|Default|Getref%20to%20Player)) (Variables|Default|GetHelpsReq))
      (CallFunction|SwordUpgrade)
      (Variables|Default|SetHelpsReq 5))))

(fn ConstructionScript)
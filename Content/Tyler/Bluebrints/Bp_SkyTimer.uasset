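; Day/night cycle manager that rotates the level's DirectionalLight, switches music and keeps a countdown for the UI.
; TimeSwap alternates Daycycle and NightCycle timelines that drive the sun's pitch, calling itself again after each day and after a delayed night hold.
; Each night increments NightNumber, and the loop stops when it reaches two.
; SkyTimer resets the countdown per phase, while a Delay on Tick decrements it each second and updates Percenttime.
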(event Custom|SkyTimer
  ;[1 1 1] Sets how long timer will last
  (if (Variables|Default|GetIsTurningNight)
    (Variables|Default|SetTime 3e+01)
    (else
      (Variables|Default|SetTime 6e+01))))

(event Custom|TimeSwap
  (bind _directionlight (Variables|Default|GetDirectionLight))
  (bind _musiccue (Variables|Default|GetMusicCue))
  (bind _musiccue_2 (Variables|Default|GetMusicCue))
  (bind _directionlight_2 (Variables|Default|GetDirectionLight))
  ;[1 1 1] Time swap function
  (Variables|Default|SetNightTimer false) ; set to day
  (if (Variables|Default|GetIsTurningNight)
    (CallFunction|SkyTimer)
    (bind _nightcycle (Timeline|NightCycle PlayFromStart) ; turns to night
      (:Update
        (Transformation|SetActorRelativeRotation _directionlight_2 (Math|Rotator|MakeRotator 0.0 _nightcycle 0.0)))
      (:Finished
        (Variables|Default|SetIsTurningNight false)
        (Class|LightComponent|SetTemperature (Variables|/Script/Engine.Light|GetLightComponent _directionlight_2) 6.5e+03) ; If we need to change temp/ color of sun during night
        (Variables|Default|SetNightTimer true) ; Is night = true is day = false
        (Math|Integer|IncrementInt (Variables|Default|GetNightNumber) ; night number up by one
          (:%20%20
            (Audio|Components|Audio|SetSound _musiccue_2 "/Game/Developers/dynod/Collections/FloodDevinChin.FloodDevinChin")
            (Audio|Components|Audio|FadeIn _musiccue_2 2.0 1.0 0.0 "Linear" :!class /Script/Engine.AudioComponent)
            (if (not (== (Variables|Default|GetNightNumber) 2))
              (Variables|Default|SetTime 6e+01) ; sets timer for night in the UI
              (Utilities|FlowControl|Delay 6e+01) ; delay for duration of night
              (CallFunction|TimeSwap :!label _label))))))
    (else
      (CallFunction|SkyTimer)
      (Audio|Components|Audio|SetSound _musiccue "/Game/Developers/dynod/Collections/SoHowDoesThatMakeYouFeelDevinChin.SoHowDoesThatMakeYouFeelDevinChin")
      (Audio|Components|Audio|FadeIn _musiccue 2.0 1.0 0.0 "Linear" :!class /Script/Engine.AudioComponent)
      (bind _daycycle (Timeline|Daycycle PlayFromStart) ; turns to day
        (:Update
          (Transformation|SetActorRelativeRotation _directionlight (Math|Rotator|MakeRotator 0.0 _daycycle 0.0)))
        (:Finished
          (Variables|Default|SetIsTurningNight true)
          (Class|LightComponent|SetTemperature (Variables|/Script/Engine.Light|GetLightComponent _directionlight) 6.5e+03) ; If we need to change temp/ color of sun during day
          (goto _label))))))

(event Custom|DaySwap
  (bind _musiccue (Variables|Default|GetMusicCue))
  (bind _musiccue_2 (Variables|Default|GetMusicCue))
  (if (Variables|Default|GetNightTimer)
    (Audio|Components|Audio|SetSound _musiccue "/Game/Developers/dynod/Collections/FloodDevinChin.FloodDevinChin")
    (Audio|Components|Audio|FadeIn _musiccue 2.0 1.0 0.0 "Linear" :!class /Script/Engine.AudioComponent)
    (else
      (Audio|Components|Audio|SetSound _musiccue_2 "/Game/Developers/dynod/Collections/SoHowDoesThatMakeYouFeelDevinChin.SoHowDoesThatMakeYouFeelDevinChin")
      (Audio|Components|Audio|FadeIn _musiccue_2 2.0 1.0 0.0 "Linear" :!class /Script/Engine.AudioComponent))))

(event EventBeginPlay
  ;[1 1 1] Ref to light and sky dome, calls timer function
  (bind _outactors (Actor|GetAllActorsOfClass "/Script/Engine.DirectionalLight"))
  (Variables|Default|SetDirectionLight (Utilities|Array|Get(acopy) _outactors))
  (CallFunction|DaySwap)
  (CallFunction|TimeSwap)
  (Utilities|FlowControl|Delay 3e+01)
  (Variables|Default|SetMaxTime 6e+01))

(event EventTick
  (params (DeltaSeconds :type Float%20%28single-precision%29))
  ;[1 1 1] Update time every second
  (Utilities|FlowControl|Delay 1.0)
  (Math|Float|DecrementFloat (Variables|Default|GetTime)
    (:%20%20
      (Variables|Default|SetPercenttime (/ (Variables|Default|GetTime) (Variables|Default|GetMaxTime))))))

(fn ConstructionScript)